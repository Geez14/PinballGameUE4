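; BP_Ball is a physics-driven ball that keeps rolling forward while being held to the surface beneath it.
; Each Tick it adds a velocity-change impulse of DefaultSpeed scaled by delta time to the Ball component.
; A short downward Visibility trace supplies the impact normal, and a second impulse pushes the ball against that normal, scaled by Stickiness and delta time, without branching on a hit.
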(event EventBeginPlay)

(event Collision|EventActorBeginOverlap
  (params (OtherActor :type Actor%20Object%20Reference)))

(event EventTick
  (params (DeltaSeconds :type Float%20%28single-precision%29))
  (bind _returnvalue (Transformation|GetActorLocation))
  (Physics|AddImpulse (Variables|Default|GetBall) (* (Variables|Default|GetDefault_speed) DeltaSeconds) "None" true)
  ;[1 1 1] To Trace the path fo the ball onto z axis
  (bind _outhit (Collision|LineTraceByChannel _returnvalue (- _returnvalue "0.000000,0.000000,500.000000") "TraceTypeQuery1" false 0 "None"))
  (Physics|AddImpulse (Variables|Default|GetBall) (* (* (.ImpactNormal (Collision|BreakHitResult _outhit)) -1.0) (* (Variables|Default|Getstickiness) DeltaSeconds)) "None" true))

(fn ConstructionScript)