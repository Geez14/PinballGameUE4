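; Pinball bumper actor that knocks the ball away and awards score when a BP_Ball overlaps it.
; Bump plays a sound, applies a mass-independent impulse outward from the bumper, and adds points through Pinball_GameMode.
; The BumpLerp timeline then drives the mechanism's vertical motion, the Blink light intensity and the emissive glow from one shared curve.
; The glow uses a dynamic material instance created on BumperBase in the construction script.
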(event Custom|Bump
  (params (Bp_ball :type BP%20Ball%20Object%20Reference))
  (Audio|PlaySound2D "/Game/Assets/Music/Bumper_sfx.Bumper_sfx" 1.0 1.0 0.0 0 0)
  (Physics|AddImpulse (Variables|/Game/Assets/bluprints/BP_Ball.BP_Ball_C|GetBall Bp_ball) (* (Math|Vector|GetUnitDirection(Vector) (Transformation|GetActorLocation) (Transformation|GetActorLocation Bp_ball)) 2.3e+03) "None" true)
  (bind _aspinball_game_mode (Utilities|Casting|CastToPinball_GameMode (Game|GetGameMode)))
  (Default|AddScore _aspinball_game_mode 1e+02)
  ;[1 1 1] parameter for mechanism
  (bind _mechanismmotion (Timeline|BumpLerp PlayFromStart)
    (:Update
      (Transformation|SetRelativeLocation (Variables|Default|GetBumper_Mechanism) (Math|Vector|Lerp(Vector) "0, 0,60.000000" "0, 0,-60.000000" _mechanismmotion) false false)
      ;[1 1 1] light blink controll using motion of bumper_mechanism
      (Rendering|Components|Light|SetIntensity (Variables|Default|GetBlink) (Math|Float|Lerp 0.0 5e+03 _mechanismmotion))
      ;[1 1 1] Construction of glowing light of top bumper
      (Rendering|Material|SetScalarParameterValue (Variables|Default|GetBumperTopMID) "EmissiveBoost" (Math|Float|Lerp 0.0 5e+01 _mechanismmotion) :!class /Script/Engine.MaterialInstanceDynamic))))

(event EventBeginPlay)

(event Collision|EventActorBeginOverlap
  (params (OtherActor :type Actor%20Object%20Reference))
  (bind _asbp_ball (Utilities|Casting|CastToBP_Ball OtherActor))
  (CallFunction|Bump _asbp_ball))

(event EventTick
  (params (DeltaSeconds :type Float%20%28single-precision%29)))

(fn ConstructionScript
  ;[1 1 1] Glow on bumper top
  (bind _returnvalue (Rendering|Material|CreateDynamicMaterialInstance (Variables|Default|GetBumper_base) 0 0 "None" :!class /Script/Engine.PrimitiveComponent))
  (Variables|Default|SetBumperTopMID _returnvalue))