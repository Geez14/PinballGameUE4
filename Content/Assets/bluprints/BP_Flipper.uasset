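; BP_Flipper is a pinball-style flipper actor that swings between a rest angle and a flipped angle.
; The construction script derives start and end rotations from Fliptype, poses the Flicker component at the start, and mirrors the Right variant with negative X scale.
; Flip and Flop custom events use MoveComponentTo to rotate Flicker to the end or back over TimeToFlip, with no triggering input inside this Blueprint.
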(event Custom|Flip
  ;[1 1 1] This is the custom event to tell the object what is meant by flip and can be call during another type of evet like when player press somthing call "Flip".
  ;[1 1 1] what to do with component(Flipper).
  ; Target is our intial position
  (Components|MoveComponentTo (Variables|Default|Getflicker) "0, 0, 0" (Variables|Default|GetEndRotation) false false (Variables|Default|GetTime%20To%20Flip) false))

(event Custom|Flop
  ;[1 1 1] This is similar to flip
  (Components|MoveComponentTo (Variables|Default|Getflicker) "0, 0, 0" (Variables|Default|GetStartRotation) false false (Variables|Default|GetTime%20To%20Flip) false))

(event EventBeginPlay)

(event Collision|EventActorBeginOverlap
  (params (OtherActor :type Actor%20Object%20Reference)))

(event EventTick
  (params (DeltaSeconds :type Float%20%28single-precision%29)))

(fn ConstructionScript
  ;[1 1 1] These are all function which is going to help to give movement to the object(in this case Flipper is object.)  : )
  ;;[1 1 1] Function creator.
  ;;[1 1 1] Here we are decrlaring rotation movement for two object belong to same blueprint class but we made two type of movement for left and right (as mirror image,because the mirrored object will have diffrent type of rotation compare to original object.)
  ;;;[1 1 1] providing array value to variable(start).
  (Variables|Default|SetStartRotation (Utilities|Select :Index (Variables|Default|GetFliptype) :NewEnumerator0 "0,20.000000, 0" :NewEnumerator1 "0,-20.000000, 0"))
  ;;;[1 1 1] providing array value to vaiable(end).
  (Variables|Default|SetEndRotation (Utilities|Select :Index (Variables|Default|GetFliptype) :NewEnumerator0 "0,-20.000000, 0" :NewEnumerator1 "0,20.000000, 0"))
  ;;[1 1 1] setting up the rotation.
  (Transformation|SetRelativeRotation (Variables|Default|Getflicker) (Variables|Default|GetStartRotation) false false)
  ;;[1 1 1] Here we are switching the position of flipper to declare what is left and right will look by rotating the object flipper.
  (switch Utilities|FlowControl|Switch|SwitchonFliptype (Variables|Default|GetFliptype)
    (:NewEnumerator1
      (Transformation|SetRelativeScale3D (Variables|Default|Getflicker) "-1.000000,1.000000,1.000000"))))